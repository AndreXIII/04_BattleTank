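; MortarWu_BP is a mortar Blueprint with a turret, a barrel and a health bar widget component.
; On BeginPlay it passes Barrel and Turret to its TankAiming component, reusing tank aiming for the mortar.
; It then casts the widget to HealthBar_BP and sets itself as MyPawn, giving the bar a reference to its owner.
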(event EventBeginPlay
  (Class|TankAimingComponent|Initialise (Variables|Default|GetTankAiming) (Variables|Default|GetBarrel) (Variables|Default|GetTurret))
  (CallFunction|InitialiseHealthBarWidget))

(fn ConstructionScript)

(fn InitialiseHealthBarWidget
  (bind _ashealth_bar_bp (Utilities|Casting|CastToHealthBar_BP (UserInterface|GetUserWidgetObject (Variables|Default|GetHealthBar)))
    (:then
      (Variables|/Game/UI/HealthBar_BP.HealthBar_BP_C|SetMyPawn _ashealth_bar_bp self))
    (:CastFailed
      _))
  (return))